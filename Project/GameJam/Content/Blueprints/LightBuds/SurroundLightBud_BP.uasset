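; SurroundLightBud_BP is a light bud variant that, judging by its name and component list, uses several boxes as surrounding light triggers.
; On BeginPlay it gathers LightBox and seven other Box components into the LightTriggers array, then calls SetupLightTriggers, whose logic is not defined in this graph.
; The construction script is empty.
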(event EventBeginPlay
  (Variables|Default|SetLightTriggers (Utilities|Array|MakeArray (Variables|Default|GetLightBox) (Variables|Default|GetBox) (Variables|Default|GetBox1) (Variables|Default|GetBox2) (Variables|Default|GetBox3) (Variables|Default|GetBox4) (Variables|Default|GetBox5) (Variables|Default|GetBox6)))
  (Class|GJLightBud|SetupLightTriggers))

(fn ConstructionScript)